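; BP_Lava is a rising lava hazard that restarts the level when the player touches it.
; After a short delay from BeginPlay it plays a warning cue, then Tick raises it by LavaSpeed at a fixed scale.
; On plane overlap with BP_PlayerCharacter, it plays a death sound through BP_GameInstance that persists across the reload.
; It subtracts the game mode's temporary score from the saved score before reopening the current level.
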(event `self.ReceiveBeginPlay`
  ;[1 1 1] Lava rising
  (`KismetSystemLibrary.Delay` 10.0)
  (set `self.LavaRising` true)
  (`GameplayStatics.PlaySoundAtLocation` "/Game/Sounds/LavaRising_Cue.LavaRising_Cue" (0.0 0.0 0.0) (struct) 1.0 1.0 0.0 null null null))

(event `self.ReceiveTick`
  (params (DeltaSeconds :type "Float (single-precision)"))
  (bind (_returnvalue_x _returnvalue_y _returnvalue_z) (`KismetMathLibrary.BreakVector` (`SceneComponent.K2_GetComponentLocation` (`self.Plane`))))
  ;[1 1 1] Lava rising
  (if (`self.LavaRising`)
    (`self.K2_SetActorTransform` (`KismetMathLibrary.MakeTransform` (`KismetMathLibrary.MakeVector` 0.0 0.0 (+ (* DeltaSeconds (`self.LavaSpeed`)) _returnvalue_z)) (struct) (10.0 10.0 1.0)))))

(event `self.Plane.OnComponentBeginOverlap`
  (params (OverlappedComponent :type "PrimitiveComponent Object Reference") (OtherActor :type "Actor Object Reference") (OtherComp :type "PrimitiveComponent Object Reference") (OtherBodyIndex :type Integer) (bFromSweep :type Boolean) (SweepResult :type "HitResult Structure (by ref)"))
  ;[1 1 1] Reset Level on Collision with Player
  (cast `/Game/Blueprints/BP_PlayerCharacter` OtherActor)
  (bind _asbp_game_instance (cast `/Game/Blueprints/BP_GameInstance` (`GameplayStatics.GetGameInstance`)))
  (`/Game/Blueprints/BP_GameInstance.PlayAudio` _asbp_game_instance "/Game/Sounds/Death_Cue.Death_Cue" 1.5 true)
  (`self.DecreasePointsOnDeath`)
  (bind _returnvalue (`GameplayStatics.GetCurrentLevelName` true))
  (`GameplayStatics.OpenLevel` (`KismetStringLibrary.Conv_StringToName` _returnvalue)))

(event `DecreasePointsOnDeath`
  ;[1 1 1] Reset to precious score on death
  (bind _asbp_game_mode (cast `/Game/Blueprints/BP_GameMode` (`GameplayStatics.GetGameMode`)))
  (bind _asbp_game_instance (cast `/Game/Blueprints/BP_GameInstance` (`GameplayStatics.GetGameInstance`)))
  (set `/Game/Blueprints/BP_GameInstance.Score` (- (`/Game/Blueprints/BP_GameInstance.Score` _asbp_game_instance) (`/Game/Blueprints/BP_GameMode.ScoreTemporary` _asbp_game_mode)) _asbp_game_instance))

(fn `UserConstructionScript`)