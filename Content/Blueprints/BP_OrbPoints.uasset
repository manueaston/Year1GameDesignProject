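; BP_OrbPoints is a score pickup that the player collects by touching it.
; When its Sphere overlaps a BP_PlayerCharacter, it destroys itself and adds ScoreValue to Score in BP_GameInstance, then to ScoreTemporary in BP_GameMode.
; It then plays Score_Cue at the world origin rather than at the orb's location.
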(event `self.Sphere.OnComponentBeginOverlap`
  (params (OverlappedComponent :type "PrimitiveComponent Object Reference") (OtherActor :type "Actor Object Reference") (OtherComp :type "PrimitiveComponent Object Reference") (OtherBodyIndex :type Integer) (bFromSweep :type Boolean) (SweepResult :type "HitResult Structure (by ref)"))
  ;[1 1 1] Increase Score
  (cast `/Game/Blueprints/BP_PlayerCharacter` OtherActor)
  (`self.K2_DestroyActor`)
  (bind _asbp_game_instance (cast `/Game/Blueprints/BP_GameInstance` (`GameplayStatics.GetGameInstance`)))
  (set `/Game/Blueprints/BP_GameInstance.Score` (+ (`/Game/Blueprints/BP_GameInstance.Score` _asbp_game_instance) (`self.ScoreValue`)) _asbp_game_instance)
  (bind _asbp_game_mode (cast `/Game/Blueprints/BP_GameMode` (`GameplayStatics.GetGameMode`)))
  (set `/Game/Blueprints/BP_GameMode.ScoreTemporary` (+ (`/Game/Blueprints/BP_GameMode.ScoreTemporary` _asbp_game_mode) (`self.ScoreValue`)) _asbp_game_mode)
  (`GameplayStatics.PlaySoundAtLocation` "/Game/Sounds/Score_Cue.Score_Cue" (0.0 0.0 0.0) (struct) 1.0 1.0 0.0 null null null))

(fn `UserConstructionScript`
  (`parent.UserConstructionScript`))