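; BP_OrbJump is a pickup orb that recharges the player's double jump, then respawns after ten seconds.
; A player character overlapping its sphere disables collision, hides the orb and clears a CanOverlap guard.
; It calls FillDoubleJump on player 0's character and plays a charge sound at world origin.
; A parallel sequence branch waits out the delay, then restores visibility, collision and the guard.
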(event `self.Sphere.OnComponentBeginOverlap`
  (params (OverlappedComponent :type "PrimitiveComponent Object Reference") (OtherActor :type "Actor Object Reference") (OtherComp :type "PrimitiveComponent Object Reference") (OtherBodyIndex :type Integer) (bFromSweep :type Boolean) (SweepResult :type "HitResult Structure (by ref)"))
  ;[1 1 1] Charge Jump and Hide Orb for 10 seconds
  (cast `/Game/Blueprints/BP_PlayerCharacter` OtherActor)
  (if (`self.CanOverlap`)
    (set `self.CanOverlap` false)
    (`self.SetActorEnableCollision` false)
    (`self.SetActorHiddenInGame` true)
    (`|ExecutionSequence`
      (:`then_0`
        (bind _asbp_player_character (cast `/Game/Blueprints/BP_PlayerCharacter` (`GameplayStatics.GetPlayerCharacter` 0)))
        (`/Game/Blueprints/BP_PlayerCharacter.Fill DoubleJump` _asbp_player_character)
        (`GameplayStatics.PlaySoundAtLocation` "/Game/Sounds/JumpCharge_Cue.JumpCharge_Cue" (0.0 0.0 0.0) (struct) 1.0 1.0 0.0 null null null))
      (:`then_1`
        (`KismetSystemLibrary.Delay` 10.0)
        (`self.SetActorHiddenInGame` false)
        (`self.SetActorEnableCollision` true)
        (set `self.CanOverlap` true)))))

(fn `UserConstructionScript`
  (`parent.UserConstructionScript`))