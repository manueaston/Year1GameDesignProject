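; Player character Blueprint handling look, yaw-relative movement, jumping with a bar-gated double jump, and pausing.
; A DoN counter, reset on landing, makes the second jump launch the character with a sound when the DoubleJump bar is full.
; Self-recalling delayed events drain or fill the bar smoothly, though nothing here calls the fill.
; Pause, when allowed, opens the pause menu widget with UI-only input.
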(event `InputAction|Pause`
  (params (Key :type "Key Structure"))
  (bind _returnvalue (`GameplayStatics.GetPlayerController` 0))
  ;[1 1 1] Pause Game
  (:`Pressed`
    (if (`self.CanPause`)
      (bind _returnvalue_2 (`|CreateWidget` "/Game/Widgets/WBP_PauseMenu.WBP_PauseMenu_C"))
      (`UserWidget.AddToViewport` _returnvalue_2 0)
      (`WidgetBlueprintLibrary.SetInputMode_UIOnlyEx` _returnvalue null)
      (set `PlayerController.bShowMouseCursor` true _returnvalue)
      (`GameplayStatics.SetGamePaused` true))))

(event `InputAxis|LookLeftRight`
  (params (AxisValue :type "Float (single-precision)"))
  ;[1 1 1] Player Character Movement Inputs
  (`self.AddControllerYawInput` AxisValue))

(event `InputAxis|MoveForwardBack`
  (params (AxisValue :type "Float (single-precision)"))
  ;[1 1 1] Player Character Movement Inputs
  (`self.AddMovementInput` (`KismetMathLibrary.GetForwardVector` (`KismetMathLibrary.MakeRotator` 0.0 0.0 (.yaw (`self.GetControlRotation`)))) AxisValue))

(event `InputAxis|LookUpDown`
  (params (AxisValue :type "Float (single-precision)"))
  ;[1 1 1] Player Character Movement Inputs
  (`self.AddControllerPitchInput` AxisValue))

(event `InputAxis|MoveLeftRight`
  (params (AxisValue :type "Float (single-precision)"))
  ;[1 1 1] Player Character Movement Inputs
  (`self.AddMovementInput` (`KismetMathLibrary.GetRightVector` (`KismetMathLibrary.MakeRotator` 0.0 0.0 (.yaw (`self.GetControlRotation`)))) AxisValue))

(event `InputAction|Jump`
  (params (Key :type "Key Structure"))
  ;[1 1 1] Player Character Movement Inputs
  (:`Pressed`
    (bind _counter (`/Engine/EditorBlueprintResources/StandardMacros.Do N` 2 :!label _label)
      (:`Exit`
        (if (== _counter 2)
          (if (== (`self.DoubleJump`) 1.0)
            (`self.Drain DoubleJump`)
            (`self.LaunchCharacter` (`KismetMathLibrary.MakeVector` 0.0 0.0 (`CharacterMovementComponent.JumpZVelocity` (`self.CharacterMovement`))) false true)
            (`GameplayStatics.PlaySoundAtLocation` "/Game/Sounds/Jump_Cue.Jump_Cue" (0.0 0.0 0.0) (struct) 1.0 1.0 0.0 null null null))
          (else
            (`self.Jump`)))))))

(event `self.OnLanded`
  (params (Hit :type "HitResult Structure (by ref)"))
  ;[1 1 1] Player Character Movement Inputs
  (goto _label :!via `Reset`))

(event `Drain DoubleJump`
  ;[1 1 1] Drain/Fill Jump Bar Smoothly
  (if (`self.ShouldDrain`)
    (bind _output_get (set `self.DoubleJump` (`KismetMathLibrary.FClamp` (- (`self.DoubleJump`) 0.1))))
    (if (== _output_get 0.0)
      (set `self.ShouldDrain` false)
      (set `self.ShouldFill` true)
      (else
        (`KismetSystemLibrary.Delay` 0.01)
        (`self.Drain DoubleJump`)))))

(event `Fill DoubleJump`
  ;[1 1 1] Drain/Fill Jump Bar Smoothly
  (if (`self.ShouldFill`)
    (bind _output_get (set `self.DoubleJump` (`KismetMathLibrary.FClamp` (+ (`self.DoubleJump`) 0.1))))
    (if (== _output_get 1.0)
      (set `self.ShouldFill` false)
      (set `self.ShouldDrain` true)
      (else
        (`KismetSystemLibrary.Delay` 0.01)
        (`self.Fill DoubleJump`)))))

(fn `UserConstructionScript`)